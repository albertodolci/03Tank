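; Player-controlled tank Blueprint that wires up aiming, firing and camera orbit input.
; On BeginPlay it hands the Barrel and Turret to the AimingC component and passes the Barrel to its own SetCannone.
; The Fire input calls Spara to shoot.
; Azimuth input yaws the Scene component and altitude input pitches the SpringArm, splitting the rotation axes across two components.
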(event `InputAction|Fire`
  (params (Key :type "Key Structure"))
  (:`Pressed`
    (`self.Spara`)))

(event `self.ReceiveBeginPlay`
  (bind _aimingc (`self.AimingC`))
  (`AimingComponent.SetCannone` _aimingc (`self.Barrel`))
  (`AimingComponent.SetTorre` _aimingc (`self.Turret`))
  (`self.SetCannone` (`self.Barrel`)))

(event `InputAxis|MoveAltitude`
  (params (AxisValue :type "Float (single-precision)"))
  (`SceneComponent.K2_AddLocalRotation` (`self.SpringArm`) (`KismetMathLibrary.MakeRotator` 0.0 AxisValue) false false))

(event `InputAxis|MoveAzimuth`
  (params (AxisValue :type "Float (single-precision)"))
  (`SceneComponent.K2_AddLocalRotation` (`self.Scene`) (`KismetMathLibrary.MakeRotator` 0.0 0.0 AxisValue) false false))

(fn `UserConstructionScript`)